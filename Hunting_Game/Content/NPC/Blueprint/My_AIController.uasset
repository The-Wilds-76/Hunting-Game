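; AI controller for NPCs that runs the BT_AI behavior tree on BeginPlay.
; Its perception component passes each updated stimulus to separate sight and hearing handlers.
; Each handler checks the stimulus's sense class and writes whether it was successfully sensed to a Blackboard bool, bCanSeePlayer for sight and bHearSound for hearing.
; The handlers do not check which actor was sensed, so any sighted target sets bCanSeePlayer.
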(event OnTargetPerceptionUpdated(AI_Per)
  (params (Actor :type Actor%20Object%20Reference) (Stimulus :type AI%20Stimulus%20Structure))
  ;[1 1 1] Perception
  (CallFunction|HandleSight Stimulus)
  (CallFunction|HandleSound Stimulus))

(event EventBeginPlay
  ;[1 1 1] Run BT
  (AI|RunBehaviorTree "/Game/NPC/Blueprint/BT_AI.BT_AI"))

(fn ConstructionScript)

(fn HandleSound
  (params (Stimulus :type AI%20Stimulus%20Structure%20%28by%20ref%29))
  (bind _returnvalue (Class|AIPerceptionSystem|GetSenseClassforStimulus Stimulus))
  (if (== _returnvalue "/Script/AIModule.AISense_Hearing")
    (AI|Components|Blackboard|SetValueasBool (AI|GetBlackboard 0) (Utilities|Name|MakeLiteralName "bHearSound") (.bSuccessfullySensed (Utilities|Struct|BreakAIStimulus Stimulus)))))

(fn HandleSight
  (params (Stimulus :type AI%20Stimulus%20Structure%20%28by%20ref%29))
  (bind _returnvalue (Class|AIPerceptionSystem|GetSenseClassforStimulus Stimulus))
  (if (== _returnvalue "/Script/AIModule.AISense_Sight")
    (AI|Components|Blackboard|SetValueasBool (AI|GetBlackboard 0) (Utilities|Name|MakeLiteralName "bCanSeePlayer") (.bSuccessfullySensed (Utilities|Struct|BreakAIStimulus Stimulus)))))