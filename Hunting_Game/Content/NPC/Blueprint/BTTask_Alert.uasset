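; Behavior Tree task for an NPC alert step that counts its executions and changes blackboard perception flags.
; Each run increments CountTest: below two it clears bHearSound, and from two onward it sets bCanSeePlayer true, with no reset shown.
; Both branches print a debug string and finish the task as failed.
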(event EventReceiveExecuteAI
  (params (OwnerController :type AI%20Controller%20Object%20Reference) (ControlledPawn :type Pawn%20Object%20Reference))
  (Variables|Default|SetcountTest (+ (Variables|Default|GetcountTest) 1))
  (if (>= (Variables|Default|GetcountTest) 2)
    (Class|BTFunctionLibrary|SetBlackboardValueasBool (Utilities|Struct|MakeBlackboardKeySelector 0 (Utilities|Name|MakeLiteralName "bCanSeePlayer")) true)
    (Development|PrintString "I'm outy")
    (AI|BehaviorTree|FinishExecute false)
    (else
      (Class|BTFunctionLibrary|SetBlackboardValueasBool (Utilities|Struct|MakeBlackboardKeySelector 0 (Utilities|Name|MakeLiteralName "bHearSound")) false)
      (Development|PrintString "no sound detected")
      (AI|BehaviorTree|FinishExecute false))))