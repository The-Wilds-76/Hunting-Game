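; Behavior tree task that makes the controlled NPC flee from the player character.
; It picks a random reachable point within a wide radius around an origin offset from the pawn, directly away from the player, and moves there with AIMoveTo.
; On success it clears the bCanSeePlayer blackboard key and finishes.
; On failure it prints a debug message and retries without finishing the task.
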(event EventReceiveExecuteAI
  (params (OwnerController :type AI%20Controller%20Object%20Reference) (ControlledPawn :type Pawn%20Object%20Reference))
  (bind _returnvalue (Transformation|GetActorLocation ControlledPawn))
  ;[1 1 1] Go contrary direction to player
  (bind _asbp_first_person_character (Utilities|Casting|CastToBP_FirstPersonCharacter (Game|GetPlayerCharacter 0) :!label _label))
  (Variables|Default|SetAs%20BP%20First%20Person%20Character _asbp_first_person_character)
  (AI|AIMoveTo ControlledPawn (.RandomLocation (AI|Navigation|GetRandomReachablePointinRadius (+ _returnvalue (* (Math|Vector|GetForwardVector (Math|Rotator|FindLookatRotation _returnvalue (Transformation|GetActorLocation (Variables|Default|GetAs%20BP%20First%20Person%20Character)))) -5e+02)) 3e+03 0 0)) 0 1.2e+02 false
    (:OnSuccess
      (Class|BTFunctionLibrary|SetBlackboardValueasBool (Utilities|Struct|MakeBlackboardKeySelector 0 (Utilities|Name|MakeLiteralName "bCanSeePlayer")) false)
      (AI|BehaviorTree|FinishExecute true))
    (:OnFail
      (Development|PrintString "failed")
      (goto _label))))